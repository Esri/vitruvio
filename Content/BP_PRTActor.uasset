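; PRT actor that generates a model from RPK rule-package data and displays it as a procedural mesh with a collision box.
; Construction regenerates when the first mesh section is not visible; BeginPlay (editor only) and ServerJoinsBeginPlay also trigger generation.
; In editor, Generate rebuilds mesh sections from the model data, with dynamic materials using textures imported from buffers.
; The construction script and server-join event save attributes after generating.
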(event Custom|SaveAttributes
  ;[1 1 1] Storing Data on Generate
  (Variables|PRT|SetAttributes (Variables|Default|GetViewAttributesDataStore)))

(event Custom|ServerJoinsBeginPlay
  (Class|PRTActor|InitializeRPKData false)
  (Class|PRTActor|Generate false)
  (CallFunction|SaveAttributes))

(event Custom|Create%20Mesh
  ;[1 1 1] Process Generated Data
  (bind (_meshstruct _bdatavalid) (Class|PRTActor|GetModelData))
  (if _bdatavalid
    (CallFunction|CreateProceduralMesh _meshstruct)
    (Class|PRTActor|SetCollisionBox (Variables|Default|GetBox))
    (else
      (Development|PrintString "Invalid Mesh Data on Generate" true true "(R=0.000000,G=0.660000,B=1.000000,A=1.000000)" 5.0))))

(event EventBeginPlay
  ;[1 1 1] Begin Play
  (if (Class|PRTActor|InEditor)
    (Class|PRTActor|InitializeRPKData false)
    (Class|PRTActor|Generate true)))

(event EventGenerate
  (params (bForceRegen :type Boolean))
  ;[1 1 1] Generate
  (Class|PRTActor|GenerateModelData bForceRegen) ; Skips Regen if Attribs unchanged or not min time between
  ;[1 1 1] Create Mesh when Generate Completed if in-editor
  (if (Class|PRTActor|InEditor)
    (CallFunction|CreateMesh)))

(fn ConstructionScript
  (Variables|Default|SetPRTStaticMesh (Variables|Default|GetStaticMesh))
  (Variables|Default|SetPRTCollisionBox (Variables|Default|GetBox))
  (Variables|Default|SetPRTProceduralMesh (Variables|Default|GetRPK%20Mesh))
  (CallFunction|Regenerate)
  (CallFunction|SaveAttributes))

(fn Regenerate
  (if (not (Class|ProceduralMeshComponent|IsMeshSectionVisible (Variables|Default|GetRPK%20Mesh)))
    (Class|PRTActor|Generate true)
    (return)))

(fn ClearMesh
  (Utilities|Array|Clear (Variables|PRT|GetTextures))
  (if (Class|ProceduralMeshComponent|IsMeshSectionVisible (Variables|Default|GetRPK%20Mesh))
    (Class|ProceduralMeshComponent|ClearAllMeshSections (Variables|Default|GetRPK%20Mesh)))
  (return))

(fn CreateProceduralMesh
  (params (Meshes :type Array%20of%20PRT%20Mesh%20Struct%20Structures))
  ;[1 1 1] Data to process?
  (if (>= (Utilities|Array|Length Meshes) 1)
    (CallFunction|ClearMesh)
    (LocalVariables|SetProceduralMeshCount 0)
    (for (_array_element _array_index) Meshes
      (CallFunction|CreateMaterialInstance _array_element _array_index)
      (Class|ProceduralMeshComponent|CreateMeshSectionLinearColor (Variables|Default|GetRPK%20Mesh) _array_index (.Vertices (Utilities|Struct|BreakPRTMeshStruct _array_element)) (.Indices (Utilities|Struct|BreakPRTMeshStruct _array_element)) (.Normals (Utilities|Struct|BreakPRTMeshStruct _array_element)) (.UVs (Utilities|Struct|BreakPRTMeshStruct _array_element)) 0 0 0 (.Colors (Utilities|Struct|BreakPRTMeshStruct _array_element)) 0 false)
      (Math|Integer|IncrementInt (LocalVariables|GetProceduralMeshCount)))
    (return)
    (else
      (return))))

(fn CreateMaterialInstance
  (params (Mesh :type PRT%20Mesh%20Struct%20Structure%20%28by%20ref%29) (ElementIndex :type Integer%20%28by%20ref%29))
  (bind _texture (Utilities|Struct|BreakPRTMeshStruct Mesh))
  (bind _returnvalue (Rendering|Material|CreateDynamicMaterialInstance (Variables|Default|GetRPK%20Mesh) ElementIndex 0 "None" :!class /Script/Engine.PrimitiveComponent))
  (Math|Integer|CompareInt (Utilities|Array|Length _texture)
    (:>
      (bind _returnvalue_2 (Class|KismetRenderingLibrary|ImportBufferasTexture2D _texture))
      (Utilities|Array|Add (Variables|PRT|GetTextures) _returnvalue_2)
      (Rendering|Material|SetTextureParameterValue _returnvalue "BaseColorMap" _returnvalue_2))
    (:==
      _)
    (:<
      _))
  (return))