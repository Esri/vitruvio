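; Actor that generates model data from an RPK via PRT and builds it into a procedural mesh with a collision box.
; Generation runs from construction and begin-play events, guarded by an RPK state machine.
; Tick polls for finished data to mesh; outside PIE, meshing is called directly because the editor has no Tick.
; Each mesh section gets a dynamic M_PRTMaster material, with any texture buffer imported as its base color.
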(event Custom|GenerateStore
  ;[1 1 1] Storing Data on Generate
  (Variables|RPKUtility|SetGeneratedDataStore (Variables|Default|GetViewAttributesDataStore)))

(event Custom|ServerJoinsBeginPlay
  ;[1 1 1] Begin Play
  (Class|PRTActor|InitializeRPKData false)
  (Class|PRTActor|Generate false)
  (CallFunction|GenerateStore))

(event Custom|CreateStaticMesh_1
  (AddComponent|AddProceduralMeshComponent false))

(event EventBeginPlay
  ;[1 1 1] Begin Play
  (Class|PRTActor|InitializeRPKData false)
  (Class|PRTActor|Generate true))

(event Collision|EventActorBeginOverlap
  (params (OtherActor :type Actor%20Object%20Reference)))

(event EventTick
  (params (DeltaSeconds :type Float%20%28single-precision%29))
  ;[1 1 1] Check State and trigger Meshing Event if Ready.
  (if (not (Variables|Default|GetbAttributesUpdated))
    (if (Class|PRTActor|CompareRPKState "GENTOMESH")
      (Class|PRTActor|ProcessGeneratedData))))

(event EventGenerate
  (params (bForceRegen :type Boolean))
  ;[1 1 1] Generate
  (if (Class|PRTActor|CompareRPKState "IDLE")
    (Class|PRTActor|GenerateModelData (or (stale EventGenerateRPK bForceRegen) bForceRegen)) ; Skips Regen if Attribs unchanged or not min time between
    ;[1 1 1] If Completed: Skips if Fire-and-Forget Task
    (if (Class|PRTActor|CompareRPKState "GENTOMESH")
      ;[1 1 1] No Tick in-Editor, so call Event.
      (if (not (Class|PRTActor|InPIE))
        (Class|PRTActor|ProcessGeneratedData)))))

(event EventProcessGeneratedData
  ;[1 1 1] Comment
  (bind _meshstruct (Class|PRTActor|GetModelData))
  (CallFunction|CreateProceduralMesh _meshstruct)
  (Class|PRTActor|SetCollisionBox)
  (Class|PRTActor|SetRPKState "IDLE"))

(event EventGenerateRPK
  (params (bForceRegen :type Boolean))
  ;[1 1 1] Generate
  (if (Class|PRTActor|CompareRPKState "IDLE")
    (Class|PRTActor|GenerateModelData (or bForceRegen (stale EventGenerate bForceRegen))) ; Skips Regen if Attribs unchanged or not min time between
    ;[1 1 1] If Completed: Skips if Fire-and-Forget Task
    (if (Class|PRTActor|CompareRPKState "GENTOMESH")
      ;[1 1 1] No Tick in-Editor, so call Event.
      (if (not (Class|PRTActor|InPIE))
        (Class|PRTActor|ProcessGeneratedData)))))

(fn ConstructionScript
  (Variables|Default|SetPRTStaticMesh (Variables|Default|GetStaticMesh))
  (Variables|Default|SetPRTCollisionBox (Variables|Default|GetBox))
  (Variables|Default|SetPRTProceduralMesh (Variables|Default|GetRPK%20Mesh))
  (CallFunction|Regenerate)
  (CallFunction|GenerateStore))

(fn Regenerate
  (if (not (Class|ProceduralMeshComponent|IsMeshSectionVisible (Variables|Default|GetRPK%20Mesh)))
    (Class|PRTActor|Generate true)
    (Class|PRTActor|ProcessGeneratedData)
    (return)))

(fn ClearMesh
  (Utilities|Array|Clear (Variables|RPKUtility|GetTextures))
  (Class|ProceduralMeshComponent|ClearAllMeshSections (Variables|Default|GetRPK%20Mesh))
  (return))

(fn CreateProceduralMesh
  (params (Array :type Array%20of%20PRT%20Mesh%20Struct%20Structures))
  (Class|PRTActor|SetRPKState "MESHING")
  (if (>= (Utilities|Array|Length Array) 1)
    (CallFunction|ClearMesh)
    (LocalVariables|SetProceduralMeshCount 0)
    (Utilities|FlowControl|Sequence
      (:then_1
        (for (_array_element _array_index) Array
          (CallFunction|CreateMaterialInstance _array_element _array_index)
          (Class|ProceduralMeshComponent|CreateMeshSectionLinearColor (Variables|Default|GetRPK%20Mesh) _array_index (.Vertices (Utilities|Struct|BreakPRTMeshStruct _array_element)) (.Indices (Utilities|Struct|BreakPRTMeshStruct _array_element)) (.Normals (Utilities|Struct|BreakPRTMeshStruct _array_element)) (.UVs (Utilities|Struct|BreakPRTMeshStruct _array_element)) 0 0 0 (.Colors (Utilities|Struct|BreakPRTMeshStruct _array_element)) 0 false)
          (LocalVariables|SetProceduralMeshCount (+ (LocalVariables|GetProceduralMeshCount) 1)))
        (Class|PRTActor|SetRPKState "MESHINGTOCOMPL")
        (Development|PrintString (Utilities|String|Append "Section Count: " (Utilities|String|ToString(Integer) (LocalVariables|GetProceduralMeshCount))) true true "(R=1.000000,G=0.133973,B=0.181746,A=1.000000)" 8.0)
        (return)))
    (else
      (Development|PrintString "No Data in MeshStruct: Skipping")
      (return))))

(fn CreateMaterialInstance
  (params (PRT%20Mesh%20Structure :type PRT%20Mesh%20Struct%20Structure%20%28by%20ref%29) (ElementIndex :type Integer))
  (bind _texture (Utilities|Struct|BreakPRTMeshStruct PRT%20Mesh%20Structure))
  (bind _returnvalue (Rendering|Material|CreateDynamicMaterialInstance (Variables|Default|GetRPK%20Mesh) ElementIndex "/PRT/M_PRTMaster.M_PRTMaster" "None" :!class /Script/Engine.PrimitiveComponent))
  (Math|Integer|CompareInt (Utilities|Array|Length _texture)
    (:>
      (bind _returnvalue_2 (Class|KismetRenderingLibrary|ImportBufferasTexture2D _texture))
      (Utilities|Array|Add (Variables|RPKUtility|GetTextures) _returnvalue_2)
      (Rendering|Material|SetTextureParameterValue _returnvalue "BaseColorMap" _returnvalue_2))
    (:==
      _)
    (:<
      _))
  (return))